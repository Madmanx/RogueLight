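; Level builder actor that, on BeginPlay, turns one of three randomly chosen Paper2D tilemaps into a 3D level.
; It walks cells on a 400-unit grid and layers in reverse, mapping tile user data to rotated piece actors.
; Start tiles place and turn the player; collectables and lasers take the last piece's rotation.
; It passes itself to the player, lasers and GTD pieces; older generators remain as unexecuted graphs.
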(event `self.ReceiveBeginPlay`
  (bind _returnvalue (`GameplayStatics.GetPlayerController` 0))
  (bind _location (`self.Location`))
  (bind _previousactorspawn (`self.PreviousActorSpawn`))
  (bind (_returnvalue_x _returnvalue_y) (`KismetMathLibrary.BreakVector` (`self.GetActorForwardVector` (`self.PreviousActorSpawn`))))
  (bind (_returnvalue_roll _returnvalue_pitch _returnvalue_yaw) (`KismetMathLibrary.BreakRotator` (`self.K2_GetActorRotation` _previousactorspawn)))
  (bind _returnvalue_2 (`self.K2_GetActorRotation` _previousactorspawn))
  (bind _returnvalue_3 (+ (`self.Location`) (0.0 0.0 -200.0)))
  ;[1 0 0] Load
  (bind _asfirst_person_character (cast `/Game/FirstPersonCPP/Blueprints/FirstPersonCharacter` (`GameplayStatics.GetPlayerCharacter` 0)))
  (set `/Game/FirstPersonCPP/Blueprints/FirstPersonCharacter.ProceduralLevelActorRef` self _asfirst_person_character)
  (bind _newparam (`self.getTilemap` (`KismetStringLibrary.Concat_StrStr` "map" (`KismetStringLibrary.Conv_IntToString` (`KismetMathLibrary.RandomIntegerInRange` 1 3)))))
  (`PaperTileMapComponent.SetTileMap` (`self.PaperTileMap`) _newparam)
  (bind _output_get (set `self.Tilemap` _newparam))
  (for _index (range (+ (`PaperTileMap.MapHeight` _output_get) 1))
    (for _index_2 (range (+ (`PaperTileMap.MapWidth` _output_get) 1))
      (`self.SetLocation` (0.0 0.0 0.0) (`KismetMathLibrary.Conv_IntToDouble` _index) (`KismetMathLibrary.Conv_IntToDouble` _index_2))
      (bind _arrayindex (`/Engine/EditorBlueprintResources/StandardMacros.ReverseForEachLoop` (`PaperTileMap.TileLayers` _output_get))
        (:`LoopBody`
          (bind _returnvalue_4 (`KismetStringLibrary.Conv_NameToString` (`TileMapBlueprintLibrary.GetTileUserData` (`PaperTileMapComponent.GetTile` (`self.PaperTileMap`) _index _index_2 _arrayindex))))
          ;[1 0.6847 0] layer1
          (switch `string` _returnvalue_4
            (:`Default`
              (switch `string` _returnvalue_4
                (:`Default`
                  (switch `string` _returnvalue_4
                    (:`Default`
                      (switch `string` _returnvalue_4
                        (:`Default`
                          (switch `string` _returnvalue_4
                            (:`Default`
                              (switch `string` _returnvalue_4
                                (:`Default`
                                  ;[0 1 0.2575] Laser/Collectables
                                  (switch `string` _returnvalue_4
                                    (:`C`
                                      (`|SpawnActorFromClass` "/Game/RogueLight/Actors/Collectable.Collectable_C" (`KismetMathLibrary.MakeTransform` (- _location (0.0 0.0 200.0)) (`KismetMathLibrary.MakeRotator` _returnvalue_roll _returnvalue_pitch (+ _returnvalue_yaw 90.0))) "Undefined" "OverrideRootScale" null null))
                                    (:`L`
                                      (bind _returnvalue_5 (`|SpawnActorFromClass` "/Game/RogueLight/Tiles/L.L_C" (`KismetMathLibrary.MakeTransform` _location _returnvalue_2) "Undefined" "OverrideRootScale" null null))
                                      (for _array_element (`self.K2_GetComponentsByClass` _returnvalue_5 "/Script/Engine.ChildActorComponent")
                                        (set `/Game/RogueLight/Actors/Laser.ProceduralLevelActor` self (cast `/Game/RogueLight/Actors/Laser` (`ChildActorComponent.ChildActor` _array_element) :!pure true))))
                                    (:`ML`
                                      (bind _returnvalue_6 (`|SpawnActorFromClass` "/Game/RogueLight/Tiles/LM.LM_C" (`KismetMathLibrary.MakeTransform` _location _returnvalue_2) "Undefined" "OverrideRootScale" null null))
                                      (for _array_element_2 (`self.K2_GetComponentsByClass` _returnvalue_6 "/Script/Engine.ChildActorComponent")
                                        (set `/Game/RogueLight/Actors/MovableLaser.ProceduralLevelActor` self (cast `/Game/RogueLight/Actors/MovableLaser` (`ChildActorComponent.ChildActor` _array_element_2) :!pure true))))))
                                (:`D`
                                  ;[0 0.5632 1] start/end fix pivot
                                  (`self.K2_SetActorLocation` (`GameplayStatics.GetPlayerPawn` 0) _returnvalue_3 false false)
                                  (set `self.Starting location` _returnvalue_3)
                                  (`|SpawnActorFromClass` "/Game/RogueLight/Tiles/S.S_C" (`KismetMathLibrary.MakeTransform` (`self.Location`) (struct)) "Undefined" "OverrideRootScale" null null)
                                  (`PlayerController.AddYawInput` _returnvalue (* _returnvalue_y 180.0))
                                  (set `self.startingRotation` (`self.K2_GetActorRotation` _returnvalue)))
                                (:`E`
                                  (`|SpawnActorFromClass` "/Game/RogueLight/Tiles/E.E_C" (`KismetMathLibrary.MakeTransform` (`self.Location`) (struct)) "Undefined" "OverrideRootScale" null null))))
                            (:`GDT`
                              (`self.spawnActor` "/Game/RogueLight/Tiles/OldStuff/GTD.GTD_C" (struct :`Yaw` 90.0))
                              (set `/Game/RogueLight/Tiles/OldStuff/GTD.ProceduralLevelActorRef` self (cast `/Game/RogueLight/Tiles/OldStuff/GTD` (`self.PreviousActorSpawn`) :!pure true) :!label _label))
                            (:`BHT`
                              (`self.spawnActor` "/Game/RogueLight/Tiles/OldStuff/GTD.GTD_C")
                              (goto _label))))
                        (:`BG`
                          (`self.spawnActor` "/Game/RogueLight/Tiles/V.V_C" (struct)))
                        (:`GH`
                          (`self.spawnActor` "/Game/RogueLight/Tiles/V.V_C" (struct :`Yaw` 90.0)))
                        (:`HD`
                          (`self.spawnActor` "/Game/RogueLight/Tiles/V.V_C" (struct :`Yaw` 180.0) (0.0 0.0 0.0)))
                        (:`DB`
                          (`self.spawnActor` "/Game/RogueLight/Tiles/V.V_C" (struct :`Yaw` 270.0)))))
                    (:`GD`
                      (`self.spawnActor` "/Game/RogueLight/Tiles/OldStuff/BH.BH_C"))
                    (:`BH`
                      (`self.spawnActor` "/Game/RogueLight/Tiles/OldStuff/BH.BH_C" (struct :`Yaw` 90.0)))))
                (:`GR`
                  (`self.spawnActor` "/Game/RogueLight/Tiles/GR.GR_C" (struct :`Yaw` 180.0) (0.0 0.0 0.0)))
                (:`HR`
                  (`self.spawnActor` "/Game/RogueLight/Tiles/GR.GR_C" (struct :`Yaw` 270.0)))
                (:`DR`
                  (`self.spawnActor` "/Game/RogueLight/Tiles/GR.GR_C" (struct)))
                (:`BR`
                  (`self.spawnActor` "/Game/RogueLight/Tiles/GR.GR_C" (struct :`Yaw` 90.0) (0.0 0.0 0.0)))))
            (:`BGH`
              (`self.spawnActor` "/Game/RogueLight/Tiles/TRI.TRI_C" (struct :`Yaw` 90.0)))
            (:`GHD`
              (`self.spawnActor` "/Game/RogueLight/Tiles/TRI.TRI_C" (struct :`Yaw` 180.0)))
            (:`HDB`
              (`self.spawnActor` "/Game/RogueLight/Tiles/TRI.TRI_C" (struct :`Yaw` 270.0)))
            (:`DBG`
              (`self.spawnActor` "/Game/RogueLight/Tiles/TRI.TRI_C" (struct)))))))))

(fn `CreateFloor`
  (params (Offset :type "Vector Structure"))
  (bind _returnvalue (`|SpawnActorFromClass` "/Script/Engine.StaticMeshActor" (`KismetMathLibrary.MakeTransform` (+ Offset (0.0 0.0 0.0)) (struct) (`self.FloorScale`)) "Undefined" "OverrideRootScale" null null))
  (bind _output_get (set `self.Element` _returnvalue))
  (`StaticMeshComponent.SetStaticMesh` (`StaticMeshActor.StaticMeshComponent` _output_get) "/Game/Geometry/Meshes/1M_Cube.1M_Cube"))

(fn `CreateWall`
  (params (WallPosition :type "Vector Structure") (WallRotation :type "Rotator Structure"))
  (bind (_floorscale_x _floorscale_y) (`KismetMathLibrary.BreakVector` (`self.FloorScale`)))
  (bind _returnvalue (`|SpawnActorFromClass` "/Script/Engine.StaticMeshActor" (`KismetMathLibrary.MakeTransform` WallPosition WallRotation (`KismetMathLibrary.MakeVector` 1.0 _floorscale_y 10.0)) "Undefined" "OverrideRootScale" null null))
  (bind _output_get (set `self.Element` _returnvalue))
  (`StaticMeshComponent.SetStaticMesh` (`StaticMeshActor.StaticMeshComponent` _output_get) "/Game/Geometry/Meshes/1M_Cube.1M_Cube"))

(fn `getTilemap`
  (params (string :type String))
  (returns (NewParam :type "PaperTileMap Object Reference"))
  (switch `string` string
    (:`map1`
      (return "/Game/RogueLight/Maps/map1.map1"))
    (:`map2`
      (return "/Game/RogueLight/Maps/map2.map2"))
    (:`map3`
      (return "/Game/RogueLight/Maps/map3.map3"))
    (:`map4`
      (return "/Game/RogueLight/Maps/map4.map4"))
    (:`map5`
      (return "/Game/RogueLight/Maps/map5.map5"))))

(fn `SetLocation`
  (params (A :type "Vector Structure") (B :type "Float (double-precision)") (B2 :type "Float (double-precision)"))
  (set `self.Location` (+ A (* (400.0 0.0 0.0) B) (* (0.0 400.0 0.0) B2))))

(fn `spawnActor`
  (params (Actor :type "Actor Class Reference") (Rotaiton :type "Rotator Structure") (Location :type "Vector Structure"))
  (bind _returnvalue (`|SpawnActorFromClass` Actor (`KismetMathLibrary.MakeTransform` (+ Location (`self.Location`)) Rotaiton) "Undefined" "OverrideRootScale" null null))
  (set `self.PreviousActorSpawn` _returnvalue))

(fn `UserConstructionScript`)